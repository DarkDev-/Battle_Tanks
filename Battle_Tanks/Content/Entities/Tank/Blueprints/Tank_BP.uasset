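; Player-controllable tank Blueprint that hands driving and gunnery to its TankMovement and TankAiming components.
; On BeginPlay it passes the barrel and turret to TankAiming and both tracks to TankMovement.
; Move, turn and fire inputs forward straight to those components.
; Aim inputs rotate only the camera rig, yawing the azimuth gimbal and pitching the spring arm separately, rather than moving the turret or barrel directly.
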(event `self.ReceiveBeginPlay`
  (`TankAimingComponent.Initialize` (`self.TankAiming`) (`self.Barrel`) (`self.Turret`))
  (`TankMovementComponent.InitializeComponents` (`self.TankMovement`) (`self.Track_Left`) (`self.Track_Right`)))

(event `InputAxis|Move Forward`
  (params (AxisValue :type "Float (single-precision)"))
  ;[1 1 1] Setup Movement Input
  (`TankMovementComponent.MoveForward` (`self.TankMovement`) AxisValue))

(event `InputAxis|AimAzimuth`
  (params (AxisValue :type "Float (single-precision)"))
  ;[1 1 1] Setup Aiming Input
  (`SceneComponent.K2_AddLocalRotation` (`self.Azimuth_Gimbal`) (`KismetMathLibrary.MakeRotator` 0.0 0.0 AxisValue) false false))

(event `InputAction|Fire`
  (params (Key :type "Key Structure"))
  ;[1 1 1] Setup Fire Input
  (:`Pressed`
    (`TankAimingComponent.Fire` (`self.TankAiming`))))

(event `InputAxis|Turn Right`
  (params (AxisValue :type "Float (single-precision)"))
  ;[1 1 1] Setup Movement Input
  (`TankMovementComponent.TurnRight` (`self.TankMovement`) AxisValue))

(event `InputAxis|AimElevation`
  (params (AxisValue :type "Float (single-precision)"))
  ;[1 1 1] Setup Aiming Input
  (`SceneComponent.K2_AddLocalRotation` (`self.SpringArm`) (`KismetMathLibrary.MakeRotator` 0.0 AxisValue) false false))

(fn `UserConstructionScript`)